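; Component that shows and removes the save-game pause menu on the player's HUD.
; TogglePause creates a SaveGameMenu, anchors it on the EMS_PC HUD canvas at PausePosition and switches input to UI only.
; RemovePause hides the cursor, clears the character's IsPaused flag, removes the menu and restores game-only input.
; Neither function pauses the world itself, and ComponentsToSave is an empty stub.
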(fn `ComponentsToSave`
  (returns (Components :type "Array of ActorComponent Object Reference"))
  (return))

(fn `RemovePause`
  (bind _returnvalue (`GameplayStatics.GetPlayerController` 0))
  (set `PlayerController.bShowMouseCursor` false _returnvalue)
  (bind _asems_character (cast `/Game/DCUP/EasyMultiSaveContent/Blueprints/GameMode/EMS_Character` (`GameplayStatics.GetPlayerCharacter` 0)))
  (set `/Game/DCUP/EasyMultiSaveContent/Blueprints/GameMode/EMS_Character.Is Paused?` false _asems_character)
  (bind _asems_pc (cast `/Game/DCUP/EasyMultiSaveContent/Blueprints/GameMode/EMS_PC` _returnvalue))
  (`PanelWidget.RemoveChild` (`/Game/DCUP/UI/W_Hud.HUD_Canvas` (`/Game/DCUP/EasyMultiSaveContent/Blueprints/GameMode/EMS_PC.HUD_Widget` _asems_pc)) (`/Game/DCUP/Core/BP_WidgetComponent.Pause Widget` (`/Game/DCUP/EasyMultiSaveContent/Blueprints/GameMode/EMS_Character.BP_WidgetComponent` _asems_character)))
  (`WidgetBlueprintLibrary.SetInputMode_GameOnly` _returnvalue))

(fn `TogglePause`
  (bind _pause_widget (`self.Pause Widget`))
  (bind _returnvalue (`|CreateWidget` "/Game/DCUP/EasyMultiSaveContent/UI/SaveGame/SaveGameMenu.SaveGameMenu_C"))
  (set `self.Pause Widget` _returnvalue)
  (bind _asems_pc (cast `/Game/DCUP/EasyMultiSaveContent/Blueprints/GameMode/EMS_PC` (`GameplayStatics.GetPlayerController` 0)))
  (bind _returnvalue_2 (`CanvasPanel.AddChildToCanvas` (`/Game/DCUP/UI/W_Hud.HUD_Canvas` (`/Game/DCUP/EasyMultiSaveContent/Blueprints/GameMode/EMS_PC.HUD_Widget` _asems_pc)) _pause_widget))
  (`CanvasPanelSlot.SetAutoSize` _returnvalue_2 true)
  (`CanvasPanelSlot.SetAlignment` _returnvalue_2 (0.5 0.5))
  (`CanvasPanelSlot.SetAnchors` _returnvalue_2 (make `Anchors` (0.3 0.3) (0.3 0.3)))
  (`CanvasPanelSlot.SetPosition` _returnvalue_2 (`self.PausePosition`))
  (`WidgetBlueprintLibrary.SetInputMode_UIOnlyEx` (`GameplayStatics.GetPlayerController` 0) _pause_widget))