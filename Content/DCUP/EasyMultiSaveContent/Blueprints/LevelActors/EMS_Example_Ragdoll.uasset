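; Example ragdoll actor for Easy Multi Save that shows how physics motion persists through saving and loading.
; An overlapping pawn turns on skeletal mesh physics and shoves it with an impulse scaled from the pawn's velocity.
; Before saving, it records the simulation state and each bone's linear and angular velocity in a struct array.
; On load, it restores the simulation state, then reapplies those velocities by bone name.
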(event `self.SkeletalMesh.OnComponentBeginOverlap`
  (params (OverlappedComponent :type "PrimitiveComponent Object Reference") (OtherActor :type "Actor Object Reference") (OtherComp :type "PrimitiveComponent Object Reference") (OtherBodyIndex :type Integer) (bFromSweep :type Boolean) (SweepResult :type "HitResult Structure (by ref)"))
  ;[1 1 1] Allow throwing ragdoll around
  (`PrimitiveComponent.SetSimulatePhysics` (`self.SkeletalMesh`) true)
  (`PrimitiveComponent.AddImpulse` OverlappedComponent (* (`self.GetVelocity` (cast `Pawn` OtherActor :!pure true)) 0.5) "None" false))

(event `EMSActorSaveInterface.ActorPreSave`
  ;[1 1 1] Save Velocity and Simulation State
  (`self.Save Ragdoll Velocity`)
  (set `self.bSimulatingPhysics` (`SceneComponent.IsAnySimulatingPhysics` (`self.SkeletalMesh`))))

(event `EMSActorSaveInterface.ActorLoaded`
  ;[1 1 1] Save Velocity and Simulation State
  (`self.Load Ragdoll Velocity`))

(event `Save Ragdoll Velocity`
  (bind _skeletalmesh (`self.SkeletalMesh`))
  ;[1 1 1] Save Velocity and Simulation State
  (for _index (range (+ (`SkinnedMeshComponent.GetNumBones` (`self.SkeletalMesh`)) 1))
    (bind _returnvalue (`SkinnedMeshComponent.GetBoneName` (`self.SkeletalMesh`) _index))
    (bind _returnvalue_2 (`PrimitiveComponent.GetPhysicsLinearVelocity` _skeletalmesh _returnvalue))
    (`KismetArrayLibrary.Array_Set` (`self.RagdollVelocity`) _index (make `/Game/DCUP/EasyMultiSaveContent/Blueprints/Structs/EMS_RagdollStruct` _returnvalue _returnvalue_2 (`PrimitiveComponent.GetPhysicsAngularVelocityInDegrees` _skeletalmesh _returnvalue)) true)))

(event `Load Ragdoll Velocity`
  (bind _skeletalmesh (`self.SkeletalMesh`))
  ;[1 1 1] Save Velocity and Simulation State
  (`PrimitiveComponent.SetSimulatePhysics` (`self.SkeletalMesh`) (`self.bSimulatingPhysics`))
  (for _array_element (`self.RagdollVelocity`)
    (bind (_bone _linearvel _angularvel) (break `/Game/DCUP/EasyMultiSaveContent/Blueprints/Structs/EMS_RagdollStruct` _array_element))
    (`PrimitiveComponent.SetPhysicsLinearVelocity` _skeletalmesh _linearvel false _bone)
    (`PrimitiveComponent.SetPhysicsAngularVelocityInDegrees` _skeletalmesh _angularvel false _bone)))

(fn `ComponentsToSave`
  (returns (Components :type "Array of ActorComponent Object Reference"))
  (return))

(fn `UserConstructionScript`)