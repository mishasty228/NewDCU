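; Example level actor for Easy Multi Save: a box with a color and a number that are restored on load.
; Construction creates a dynamic material on the cube, and SetRandomColor applies a random color and number to it and its text render.
; Both setters record their values in saved variables, which ActorLoaded reapplies to rebuild the visuals.
; ComponentsToSave returns no components.
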(event `Set Random Color`
  ;[1 1 1] Box Color
  (`self.Set Box Color` (`/Game/DCUP/EasyMultiSaveContent/Blueprints/EMS_ExampleFunctions.RandomColor`))
  (`self.Set Box Text Number` (`KismetMathLibrary.RandomIntegerInRange` 1 1000)))

(event `EMSActorSaveInterface.ActorLoaded`
  ;[1 1 1] Box Color
  (`self.Set Box Color` (`self.SavedBoxColor`))
  (`self.Set Box Text Number` (`self.SavedNumber`)))

(fn `ComponentsToSave`
  (returns (Components :type "Array of ActorComponent Object Reference"))
  (return))

(fn `Set Box Color`
  (params (Color :type "LinearColor Structure"))
  (`MaterialInstanceDynamic.SetVectorParameterValue` (`self.BoxMaterial`) "Color" Color)
  (set `self.SavedBoxColor` Color))

(fn `Set Box Text Number`
  (params (Number :type Integer))
  (`TextRenderComponent.K2_SetText` (`self.TextRender`) (`KismetTextLibrary.Conv_IntToText` Number))
  (set `self.SavedNumber` Number))

(fn `UserConstructionScript`
  (bind _returnvalue (`PrimitiveComponent.CreateDynamicMaterialInstance` (`self.Cube`) 0 null "None"))
  (set `self.BoxMaterial` _returnvalue))