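; Example level actor for the Easy Multi Save plugin that demonstrates saving and loading complex nested structs on itself and its components.
; Before saving, it fills its own struct array and the one on Comp1 with example structs and gives Comp0 a random integer.
; ComponentsToSave registers both components with the save system.
; On load, it prints sample nested values from the actor and both components to verify the restored data.
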(event `EMSActorSaveInterface.ActorPreSave`
  ;[1 1 1] Save/Load a complex struct and print the data to the screen
  (for _index (range 11)
    (`KismetArrayLibrary.Array_Set` (`self.StructArray`) _index (`/Game/DCUP/EasyMultiSaveContent/Blueprints/EMS_ExampleFunctions.MakeEMSExampleStruct`) true)
    (`KismetArrayLibrary.Array_Set` (`/Game/DCUP/EasyMultiSaveContent/Blueprints/Other/EMS_ExampleActorComp.StructArray` (`self.Comp1`)) _index (`/Game/DCUP/EasyMultiSaveContent/Blueprints/EMS_ExampleFunctions.MakeEMSExampleStruct`) true))
  (set `/Game/DCUP/EasyMultiSaveContent/Blueprints/Other/EMS_ExampleActorComp.TestInt` (`KismetMathLibrary.RandomIntegerInRange` 5 10000) (`self.Comp0`)))

(event `Print Struct`
  (bind (_output_testbool _output_testint) (break `/Game/DCUP/EasyMultiSaveContent/Blueprints/Structs/EMS_ExampleStruct` (`|GetArrayItem` (`self.StructArray`) 7)))
  (bind (_output_testbool_2 _output_testint_2 _output_teststring _output_testfloat _output_teststruct _output_teststructarray) (break `/Game/DCUP/EasyMultiSaveContent/Blueprints/Structs/EMS_ExampleStruct` (`|GetArrayItem` (`/Game/DCUP/EasyMultiSaveContent/Blueprints/Other/EMS_ExampleActorComp.StructArray` (`self.Comp1`)) 3)))
  ;[1 1 1] Save/Load a complex struct and print the data to the screen
  (`KismetSystemLibrary.PrintString` (`KismetStringLibrary.Concat_StrStr` "Comp 0 TestInt: " (`KismetStringLibrary.Conv_IntToString` (`/Game/DCUP/EasyMultiSaveContent/Blueprints/Other/EMS_ExampleActorComp.TestInt` (`self.Comp0`)))))
  (`KismetSystemLibrary.PrintString` (`KismetStringLibrary.Concat_StrStr` "Comp 1 StructArray: " (`KismetStringLibrary.Conv_IntToString` (`|GetArrayItem` (`.InventoryIntArray_27_ED0AE4F24848B12441CE798B9398806C` (break `/Game/DCUP/EasyMultiSaveContent/Blueprints/Structs/EMS_IntStruct` (`|GetArrayItem` _output_teststructarray 2))) 1))))
  (`KismetSystemLibrary.PrintString` (`KismetStringLibrary.BuildString_Int` "" "StructArray: " _output_testint)))

(event `EMSActorSaveInterface.ActorLoaded`
  ;[1 1 1] Save/Load a complex struct and print the data to the screen
  (`self.Print Struct`))

(fn `ComponentsToSave`
  (returns (Components :type "Array of ActorComponent Object Reference"))
  (return (`|MakeArray` (`self.Comp0`) (`self.Comp1`) :!type "ActorComponent Object Reference")))

(fn `UserConstructionScript`)