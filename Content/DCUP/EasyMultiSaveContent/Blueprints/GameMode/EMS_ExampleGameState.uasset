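; Example game state for the EasyMultiSave (EMS) plugin that demonstrates saving and loading a very complex nested struct.
; Before saving, it fills a struct array with owned-actor entries, each pairing the pickup class with an example data struct.
; After loading, it prints an integer from deep inside the second entry's nested arrays.
; Its components-to-save function returns no components.
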(event `EMSActorSaveInterface.ActorPreSave`
  (bind _ems_ownedactorstruct (make `/Game/DCUP/EasyMultiSaveContent/Blueprints/Structs/EMS_OwnedActorStruct` "/Game/DCUP/EasyMultiSaveContent/Blueprints/Pickup/EMS_Pickup.EMS_Pickup_C" (`/Game/DCUP/EasyMultiSaveContent/Blueprints/EMS_ExampleFunctions.MakeEMSExampleStruct`)))
  ;[1 1 1] Save and Load a very complex struct
  (set `self.Struct` (`|MakeArray` _ems_ownedactorstruct _ems_ownedactorstruct _ems_ownedactorstruct)))

(event `EMSActorSaveInterface.ActorLoaded`
  ;[1 1 1] Save and Load a very complex struct
  (`KismetSystemLibrary.PrintString` (`KismetStringLibrary.Concat_StrStr` "Game State Struct:  " (`KismetStringLibrary.Conv_IntToString` (`|GetArrayItem` (`.InventoryIntArray_27_ED0AE4F24848B12441CE798B9398806C` (break `/Game/DCUP/EasyMultiSaveContent/Blueprints/Structs/EMS_IntStruct` (`|GetArrayItem` (`.TestStructArray_65_9CBAF9C5410752FBA81876B8659B339B` (break `/Game/DCUP/EasyMultiSaveContent/Blueprints/Structs/EMS_ExampleStruct` (`.ActorDataStruct_12_D61A87B04A5FB48FEEAFCEAE60425F31` (break `/Game/DCUP/EasyMultiSaveContent/Blueprints/Structs/EMS_OwnedActorStruct` (`|GetArrayItem` (`self.Struct`) 1)))))))))))))

(fn `ComponentsToSave`
  (returns (Components :type "Array of ActorComponent Object Reference"))
  (return))

(fn `UserConstructionScript`)