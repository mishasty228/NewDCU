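; BP_EnemyBase is an enemy base Blueprint with health, damage handling and a widget-based health bar.
; On BeginPlay or UpdateEnemy, it passes itself to the W_EnemyHealthBar in its HealthBar component.
; Take Damage clamps Health between zero and MaxHealth, derives HealthPercentage from a fixed divisor of 100 rather than MaxHealth, and destroys the actor at zero.
; ComponentsToSave is an empty stub.
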(event `UpdateEnemy`
  (bind _asw_enemy_health_bar (cast `/Game/DCUP/UI/W_EnemyHealthBar` (`WidgetComponent.GetUserWidgetObject` (`self.HealthBar`)) :!label _label))
  (set `/Game/DCUP/UI/W_EnemyHealthBar.BP_Enemy` self _asw_enemy_health_bar))

(event `self.ReceiveBeginPlay`
  (goto _label))

(event `self.ReceiveTick`
  (params (DeltaSeconds :type "Float (single-precision)")))

(fn `ComponentsToSave`
  (returns (Components :type "Array of ActorComponent Object Reference"))
  (return))

(fn `Take Damage`
  (params (Damage :type "Float (double-precision)"))
  (bind _output_get (set `self.Health` (`KismetMathLibrary.FClamp` (- (`self.Health`) Damage) 0.0 (`self.MaxHealth`))))
  (set `self.HealthPercentage` (/ _output_get 100.0))
  (if (== (`self.Health`) 0.0)
    (`KismetSystemLibrary.PrintString` "i died")
    (`self.K2_DestroyActor`)))

(fn `UserConstructionScript`)